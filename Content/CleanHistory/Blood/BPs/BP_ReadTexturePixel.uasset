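; Debug Blueprint that displays how much blood fills the render target of one hardcoded floor, TemplateFloor_18.
; On BeginPlay it caches the ProtoLineTracing actor, whose MapNameToRT map supplies that render target by name.
; Each tick it passes the target to GetBloodQuantityFromRenderTarget and prints the result on screen as a percentage.
; Disconnected leftover nodes hold earlier experiments with nested loops and per-pixel render target reads.
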(event `self.ReceiveBeginPlay`
  (`|ExecutionSequence`
    (:`then_0`
      (bind _returnvalue (`GameplayStatics.GetActorOfClass` "/Game/CleanHistory/Blood/BPs/ProtoLineTracing.ProtoLineTracing_C"))
      (set `self.ProtoLineTracing` _returnvalue))))

(event `self.ReceiveTick`
  (params (DeltaSeconds :type "Float (single-precision)"))
  (bind (_value _returnvalue) (`BlueprintMapLibrary.Map_Find` (`/Game/CleanHistory/Blood/BPs/ProtoLineTracing.MapNameToRT` (`self.ProtoLineTracing`)) "TemplateFloor_18"))
  (if _returnvalue
    (bind _returnvalue_2 (`self.GetBloodQuantityFromRenderTarget` _value))
    (`KismetSystemLibrary.PrintString` (`KismetStringLibrary.Concat_StrStr` "Render Target : TemplateFloor_18 is filled to " (`KismetStringLibrary.Conv_Int64ToString` (`KismetMathLibrary.Conv_DoubleToInt64` (* _returnvalue_2 100.0))) "% of blood") true true (struct :`R` 1.0 :`G` 0.116728 :`A` 1.0) DeltaSeconds)))

(fn `UserConstructionScript`)