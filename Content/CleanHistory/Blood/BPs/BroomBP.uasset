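; Broom actor for cleaning, which delegates its draw-and-wash behavior and its own cleaning to a DrawAndWash component.
; BeginPlay registers Root2 as that component's only raycast root; unconnected nodes hold alternative multi-root and self-ignore setups.
; The CleanBroom event cleans the broom by PercentageCleanedByWash, while BPCleanBroom uses a hardcoded amount.
; A getter exposes the GrabComponent's world transform.
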(event `self.ReceiveBeginPlay`
  (`KismetArrayLibrary.Array_Add` (`/Game/CleanHistory/Blood/BPs/DrawAndWash.RootTarget` (`self.DrawAndWash`)) (`self.Root 2`)))

(event `self.CleanBroom`
  (`/Game/CleanHistory/Blood/BPs/DrawAndWash.CleanBroom` (`self.DrawAndWash`) (`self.PercentageCleanedByWash`)))

(fn `BPCleanBroom`
  (`/Game/CleanHistory/Blood/BPs/DrawAndWash.CleanBroom` (`self.DrawAndWash`) 25.0))

(fn `Get Grab Component Transform`
  (returns (GrabComponent :type "Transform Structure"))
  (return (`SceneComponent.K2_GetComponentToWorld` (`self.GrabComponent`))))

(fn `UserConstructionScript`)