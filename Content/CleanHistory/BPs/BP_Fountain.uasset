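; Fountain actor that plays a water sound and pays out a one-time burst of coins when an Ecu actor touches its water.
; The first overlap drives two timelines, one animating halo material opacity and one firing coin events, then clears a boolean gate.
; Each event spawns an Ecu in a random ring around the fountain, pushes it upward with random horizontal force scaled by Expulsion, and prints debug text.
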(event `self.ReceiveBeginPlay`
  (`GameplayStatics.PlaySoundAtLocation` "/Game/CleanHistory/AUDIO/SFX/SFX_Water_Fountain_Lp_Cue.SFX_Water_Fountain_Lp_Cue" (`self.K2_GetActorLocation` self) (struct) 0.6 1.0 0.0 null null null null))

(event `self.WaterCollision.OnComponentBeginOverlap`
  (params (OverlappedComponent :type "PrimitiveComponent Object Reference") (OtherActor :type "Actor Object Reference") (OtherComp :type "PrimitiveComponent Object Reference") (OtherBodyIndex :type Integer) (bFromSweep :type Boolean) (SweepResult :type "HitResult Structure (by ref)"))
  (bind _returnvalue (`KismetMathLibrary.RandomFloatInRange` -90.0 90.0))
  (bind _returnvalue_2 (`KismetMathLibrary.RandomFloatInRange` 75.0 100.0))
  (bind _returnvalue_3 (`self.K2_GetActorLocation`))
  (bind _expulsion (`self.expulsion`))
  (bind _returnvalue_4 (`KismetMathLibrary.DegreesToRadians` (`KismetMathLibrary.RandomFloatInRange` 0.0 360.0)))
  (bind _returnvalue_5 (`KismetMathLibrary.MakeVector` (+ (* _returnvalue_2 (`KismetMathLibrary.Sin` _returnvalue_4)) (.x _returnvalue_3)) (+ (* (`KismetMathLibrary.Cos` _returnvalue_4) _returnvalue_2) (.y _returnvalue_3))))
  (cast `/Game/CleanHistory/BPs/Ecu` OtherActor)
  (if (`self.bool`)
    (`|ExecutionSequence`
      (:`then_0`
        (bind (_direction _halotrack) (`Timeline|haloTimeLine`)
          (:`Update`
            (`MeshComponent.SetScalarParameterValueOnMaterials` (`self.Halo`) "OpacityMultiplier" _halotrack))))
      (:`then_1`
        (`Timeline|Instance Coins`
          (:`Coins`
            (`KismetSystemLibrary.PrintString` "coin" true true (struct :`R` 0.10943 :`G` 0.260417 :`B` 0.215665 :`A` 1.0) 5.0)
            (bind _returnvalue_6 (`|SpawnActorFromClass` "/Game/CleanHistory/BPs/Ecu.Ecu_C" (`KismetMathLibrary.MakeTransform` _returnvalue_5 (`KismetMathLibrary.MakeRotator` _returnvalue _returnvalue _returnvalue)) "Undefined" "MultiplyWithRoot" null null))
            (`KismetSystemLibrary.PrintString` (`KismetSystemLibrary.GetDisplayName` _returnvalue_6))
            (`PrimitiveComponent.AddForce` (`/Game/CleanHistory/BPs/Ecu.StaticMesh` _returnvalue_6) (`KismetMathLibrary.MakeVector` (* (.x (- _returnvalue_5 _returnvalue_3)) _expulsion -0.005) (* (.y (- _returnvalue_5 _returnvalue_3)) _expulsion -0.005) _expulsion) "None" false))))
      (:`then_2`
        (set `self.bool` false)))))

(fn `UserConstructionScript`)