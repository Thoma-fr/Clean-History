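; Torch that lights from a burning Brasero and attaches fire ribbon effects to props or burnable actors it overlaps while lit.
; Igniting resets its burnable-object count, shows the flame mesh and plays a sound.
; Tick hides the flame when that count reaches zero but clears SetBurning, not IsBurning; nothing here decrements the count.
; The timeline-scaled extinguish and reignite feedback is disconnected and never runs.
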(event `CustomEvent`
  (params (DeltaSeconds :type "Float (single-precision)"))
  ;[1 1 1] More FeedBack on turn on and off, but no time and idc
)

(event `self.ReceiveBeginPlay`
  (set `self.IsBurning` (`self.SetBurning`)) ; not burning at the beginning
  (set `self.DefaultBurnableObject` (`self.NbBurnbaleObject`))
  (`SceneComponent.SetVisibility` (`self.FireMesh_0`) (`self.SetBurning`) true))

(event `self.CollisionBoxComponent.OnComponentBeginOverlap`
  (params (OverlappedComponent :type "PrimitiveComponent Object Reference") (OtherActor :type "Actor Object Reference") (OtherComp :type "PrimitiveComponent Object Reference") (OtherBodyIndex :type Integer) (bFromSweep :type Boolean) (SweepResult :type "HitResult Structure (by ref)"))
  (if (`self.IsBurning`)
    ;[1 1 1] Spawn Particles IsBurning
    (bind _asbp_prop (cast `/Game/CleanHistory/BPs/BP_Prop` OtherActor)
      (:`then`
        (bind _returnvalue (`NiagaraFunctionLibrary.SpawnSystemAttached` "/Game/GA/fx/fire/ribon_fire/fire_ribbon.fire_ribbon" (`/Game/CleanHistory/BPs/BP_Prop.GrabComponent` _asbp_prop) "None" (0.0 0.0 0.0) (struct) "KeepRelativeOffset"))
        (add `Prop.OnDieDelegate` _asbp_prop (delegate `OnDieDelegate_Event`)))
      (:`CastFailed`
        (cast `IBurnable` OtherActor)
        (`NiagaraFunctionLibrary.SpawnSystemAttached` "/Game/GA/fx/fire/ribon_fire/fire_ribbon.fire_ribbon" (`Actor.RootComponent` OtherActor) "None" (0.0 0.0 0.0) (struct) "KeepRelativeOffset" true true "AutoRelease")))
    (else
      ;[1 1 1] Burn if brasero or torch is burning
      (bind _asbrasero (cast `Brasero` OtherActor))
      (if (`Brasero.IsBurning` _asbrasero)
        (set `self.NbBurnbaleObject` (`self.DefaultBurnableObject`))
        (set `self.IsBurning` true)
        (`SceneComponent.SetVisibility` (`self.FireMesh_0`) true true)
        (if (`KismetSystemLibrary.IsValid` (`self.FireExstinctSound`))
          (`GameplayStatics.PlaySoundAtLocation` (`self.IgniteTorch`) (0.0 0.0 0.0) (struct) 1.0 1.0 0.0 null null null null))))))

(event `OnDieDelegate_Event`
  ;[1 1 1] Spawn Particles IsBurning
  (`ActorComponent.K2_DestroyComponent` (stale `self.CollisionBoxComponent.OnComponentBeginOverlap` _returnvalue)))

(event `self.ReceiveTick`
  (params (DeltaSeconds :type "Float (single-precision)"))
  ;[1 1 1] Extinguishing
  (if (<= (`self.NbBurnbaleObject`) 0)
    (`SceneComponent.SetVisibility` (`self.FireMesh_0`) false true)
    (set `self.SetBurning` false)))

(fn `ChangeMobilityMode`
  (params (ChangeToNotStatic :type Boolean) (NewMobility :type "EComponentMobility Enum" :default "Static"))
  (locals (NewLocalVar :type "EDOFMode Enum" :default "SixDOF"))
  (`SceneComponent.SetMobility` (`self.StaticMeshComponent`) NewMobility))

(fn `Get Grab Component Transform`
  (returns (GrabComponent :type "Transform Structure"))
  (return))

(fn `UserConstructionScript`)