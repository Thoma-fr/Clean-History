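; BP_Brasero is a burning brazier that flares up when corpse members enter it and can burn out.
; It plays a fire sound on BeginPlay.
; CorpseMembers overlapping the collision box trigger a delayed Niagara flame burst, with a DoOnce and delay limiting repeats.
; Tick polls the burnable-object count, which this graph never changes, and at zero plays an extinguish sound and timeline-shrinks the fire mesh until hidden.
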(event `self.ReceiveTick`
  (params (DeltaSeconds :type "Float (single-precision)"))
  (bind _firemesh (`self.FireMesh`))
  (bind _fireexstinctsound (`self.FireExstinctSound`))
  (if (<= (`self.NbBurnbaleObject`) 0)
    (if (`KismetSystemLibrary.IsValid` _fireexstinctsound)
      (`GameplayStatics.PlaySoundAtLocation` _fireexstinctsound (0.0 0.0 0.0) (struct) 1.0 1.0 0.0 null null null null)
      (bind (_direction _newtrack_0) (`Timeline|FadeOutTimeline` :!label _label)
        (:`Update`
          (`SceneComponent.SetWorldScale3D` (`self.FireMesh`) (* (`SceneComponent.K2_GetComponentScale` (`self.FireMesh`)) _newtrack_0)))
        (:`Finished`
          (`SceneComponent.SetWorldScale3D` _firemesh (0.0 0.0 0.0))
          (`SceneComponent.SetVisibility` _firemesh false true)))
      (else
        (goto _label)))))

(event `self.ReceiveBeginPlay`
  (`GameplayStatics.PlaySoundAtLocation` "/Game/CleanHistory/AUDIO/SFX/SFX_Fire_Lp_Cue.SFX_Fire_Lp_Cue" (`SceneComponent.K2_GetComponentLocation` (`self.FireMesh`)) (struct) 0.35 1.0 0.0 null null null null)
  (set `self.IsBurning` true))

(event `self.CollisionBoxComponent.OnComponentBeginOverlap`
  (params (OverlappedComponent :type "PrimitiveComponent Object Reference") (OtherActor :type "Actor Object Reference") (OtherComp :type "PrimitiveComponent Object Reference") (OtherBodyIndex :type Integer) (bFromSweep :type Boolean) (SweepResult :type "HitResult Structure (by ref)"))
  (cast `CorpseMembers` OtherActor)
  (`/Engine/EditorBlueprintResources/StandardMacros.DoOnce` false :!label _label_2
    (:`Completed`
      (`KismetSystemLibrary.Delay` (`self.DelayBeforeBurstParticles`))
      (`ActorComponent.Activate` (`self.NiagaraBurstFlame`) false)
      (`KismetSystemLibrary.Delay` (`self.SafeDelayBeforeNewParticles`))
      (goto _label_2 :!via `Reset`))))

(fn `UserConstructionScript`)