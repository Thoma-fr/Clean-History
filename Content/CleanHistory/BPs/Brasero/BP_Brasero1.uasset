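; BP_Brasero1 is a burning brazier that flares up when corpse parts enter it.
; On BeginPlay it plays a fire loop sound at its mesh location and sets IsBurning.
; A CorpseMembers overlap on the collision box activates a Niagara burst flame after a delay, with a DoOnce reset after a second delay to throttle repeated bursts.
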(event `self.ReceiveBeginPlay`
  (`GameplayStatics.PlaySoundAtLocation` "/Game/CleanHistory/AUDIO/SFX/SFX_Fire_Lp_Cue.SFX_Fire_Lp_Cue" (`SceneComponent.K2_GetComponentLocation` (`self.StaticMeshComponent`)) (struct) 0.35 1.0 0.0 null null null null)
  (set `self.IsBurning` true))

(event `self.CollisionBoxComponent.OnComponentBeginOverlap`
  (params (OverlappedComponent :type "PrimitiveComponent Object Reference") (OtherActor :type "Actor Object Reference") (OtherComp :type "PrimitiveComponent Object Reference") (OtherBodyIndex :type Integer) (bFromSweep :type Boolean) (SweepResult :type "HitResult Structure (by ref)"))
  (cast `CorpseMembers` OtherActor)
  (`/Engine/EditorBlueprintResources/StandardMacros.DoOnce` false :!label _label
    (:`Completed`
      (`KismetSystemLibrary.Delay` (`self.DelayBeforeBurstParticles`))
      (`ActorComponent.Activate` (`self.NiagaraBurstFlame`) false)
      (`KismetSystemLibrary.Delay` (`self.SafeDelayBeforeNewParticles`))
      (goto _label :!via `Reset`))))

(fn `UserConstructionScript`)