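; Weapon Blueprint that supplies impact sound and effect feedback when it hits something.
; PlayHit ignores impacts at or below a speed threshold, then treats skeletal meshes as bodies with a corpse sound at world origin and a blood burst at the hit point.
; Other surfaces play a floor sound at the actor and set HasHit, which Tick clears through a delay but PlayHit never checks.
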(event `self.ReceiveTick`
  (params (DeltaSeconds :type "Float (single-precision)"))
  (`KismetSystemLibrary.Delay` 2.0)
  (set `self.HasHit` false))

(fn `PlayHit`
  (params (AudioToplay :type "SoundBase Object Reference") (Vel :type "Float (double-precision)") (Hited :type "PrimitiveComponent Object Reference") (HitPos :type "Vector Structure"))
  (if (> Vel 100.0)
    (cast `SkeletalMeshComponent` Hited
      (:`then`
        (`GameplayStatics.PlaySoundAtLocation` (`self.CorpsHit`) (0.0 0.0 0.0) (struct) 1.0 1.0 0.0 null null null null)
        (`NiagaraFunctionLibrary.SpawnSystemAtLocation` "/Game/GA/fx/blood/burst/Blood_burst.Blood_burst" HitPos))
      (:`CastFailed`
        (`GameplayStatics.PlaySoundAtLocation` (`self.FloorHit`) (`self.K2_GetActorLocation`) (struct) 1.0 1.0 0.0 null null null null)
        (set `self.HasHit` true)))))

(fn `UserConstructionScript`)