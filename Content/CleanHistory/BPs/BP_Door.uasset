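; BP_Door is a door actor that swings open when its linked Brasero reports a key item burned.
; It binds to the Brasero's OnKeyItemBurn event on BeginPlay and sets ShouldOpen for any item name; OpenDoor sets the same flag.
; Tick then plays a timeline that yaws the Pivot, plays the open sound once on the first update, and sets HasOpen when finished.
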(event `self.ReceiveBeginPlay`
  ;[1 1 1] Kill me, en gros je sub la delegate a l'event
  (add `Brasero.OnKeyItemBurn` (`self.Brasero`) (delegate `OnKeyItemBurn_Event`)))

(event `OnKeyItemBurn_Event`
  (params (ItemName :type Name))
  ;[1 1 1] Kill me, en gros je sub la delegate a l'event
  (set `self.ShouldOpen` true))

(event `self.ReceiveTick`
  (params (DeltaSeconds :type "Float (single-precision)"))
  (if (`self.ShouldOpen`)
    (if (not (`self.has open`))
      (bind (_direction _rotation) (`Timeline|oipen`)
        (:`Update`
          (`SceneComponent.K2_SetRelativeRotation` (`self.pivot`) (`KismetMathLibrary.MakeRotator` 0.0 0.0 _rotation) false false)
          (`/Engine/EditorBlueprintResources/StandardMacros.DoOnce` false
            (:`Completed`
              (`GameplayStatics.PlaySoundAtLocation` (`self.DoorOpenSound`) (`SceneComponent.K2_GetComponentLocation` (`self.StaticMesh`)) (struct) 1.0 1.0 0.0 null null null null))))
        (:`Finished`
          (set `self.has open` true))))))

(fn `OpenDoor`
  (set `self.ShouldOpen` true))

(fn `UserConstructionScript`)