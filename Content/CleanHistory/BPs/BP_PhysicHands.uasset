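; Physics-driven VR hands actor that makes hand meshes follow motion controllers through physics handles.
; Setup stores both controllers and starts the grabs, though the right grab has no component specified.
; Tick drives the left handle to its controller's location and rotation; the right follows location only, with a hard-coded rotation.
; Physical animation setup for orientation strength on both hands exists but is unconnected and never runs.
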(event `self.ReceiveBeginPlay`)

(event `self.ReceiveTick`
  (params (DeltaSeconds :type "Float (single-precision)"))
  (bind _returnvalue_location (`KismetMathLibrary.BreakTransform` (`SceneComponent.K2_GetComponentToWorld` (`self.RightMotionController`))))
  (bind (_returnvalue_location_2 _returnvalue_rotation) (`KismetMathLibrary.BreakTransform` (`SceneComponent.K2_GetComponentToWorld` (`self.LeftMotionController`))))
  (`PhysicsHandleComponent.SetTargetLocationAndRotation` (`self.PhysicsHandleLeft`) _returnvalue_location_2 _returnvalue_rotation)
  (`PhysicsHandleComponent.SetTargetLocationAndRotation` (`self.PhysicsHandleRight`) _returnvalue_location (struct :`Pitch` 25.0 :`Roll` -89.0)))

(fn `Setup`
  (params (LeftMotionController :type "MotionControllerComponent Object Reference") (RightMotionController :type "MotionControllerComponent Object Reference"))
  (bind _handleft (`self.HandLeft`))
  (bind (_returnvalue_location _returnvalue_rotation) (`KismetMathLibrary.BreakTransform` (`SceneComponent.K2_GetComponentToWorld` _handleft)))
  (bind (_returnvalue_location_2 _returnvalue_rotation_2) (`KismetMathLibrary.BreakTransform` (`SceneComponent.K2_GetComponentToWorld` (`self.HandRight`))))
  (set `self.LeftMotionController` LeftMotionController)
  (set `self.RightMotionController` RightMotionController)
  (`PhysicsHandleComponent.GrabComponentAtLocationWithRotation` (`self.PhysicsHandleLeft`) _handleft "None" _returnvalue_location _returnvalue_rotation)
  (`PhysicsHandleComponent.GrabComponentAtLocationWithRotation` (`self.PhysicsHandleRight`) null "None" _returnvalue_location_2 _returnvalue_rotation_2))

(fn `UserConstructionScript`)