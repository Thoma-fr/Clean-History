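; BP_dirtHole is a diggable hole actor that responds to objects overlapping its Box.
; A Shovel overlap, after a short delay, lowers the Scene's Z scale and spawns a BP_DirtDrop at DirtDropPoint or uniformly grows the existing one.
; An overlapping BP_DirtDrop resets the Scene to full scale and is destroyed.
; Overlapping CorpseMembers make the Fill component ignore their collision channel.
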(event `self.Box.OnComponentBeginOverlap`
  (params (OverlappedComponent :type "PrimitiveComponent Object Reference") (OtherActor :type "Actor Object Reference") (OtherComp :type "PrimitiveComponent Object Reference") (OtherBodyIndex :type Integer) (bFromSweep :type Boolean) (SweepResult :type "HitResult Structure (by ref)"))
  (bind _scene (`self.Scene`))
  (bind _dirtdrop (`self.DirtDrop`))
  (bind _cube (`/Game/CleanHistory/BPs/BP_DirtDrop.Cube` _dirtdrop))
  (bind (_relativescale3d_x _relativescale3d_y _relativescale3d_z) (`KismetMathLibrary.BreakVector` (`SceneComponent.RelativeScale3D` _scene)))
  (bind (_returnvalue_x _returnvalue_y _returnvalue_z) (`KismetMathLibrary.BreakVector` (`SceneComponent.K2_GetComponentScale` _cube)))
  (bind _returnvalue (`KismetMathLibrary.FClamp` (+ _returnvalue_z (`self.DigAmount`)) 0.01 0.5))
  (cast `/Game/CleanHistory/BPs/Shovel` OtherActor
    (:`then`
      (`KismetSystemLibrary.Delay` 0.5)
      (`SceneComponent.SetRelativeScale3D` _scene (`KismetMathLibrary.MakeVector` _relativescale3d_x _relativescale3d_y (`KismetMathLibrary.FClamp` (- _relativescale3d_z (`self.DigAmount`)) 0.01)))
      (if (`KismetSystemLibrary.IsValid` _dirtdrop)
        (`SceneComponent.SetWorldScale3D` _cube (`KismetMathLibrary.MakeVector` _returnvalue _returnvalue _returnvalue))
        (else
          (bind _returnvalue_2 (`|SpawnActorFromClass` "/Game/CleanHistory/BPs/BP_DirtDrop.BP_DirtDrop_C" (`SceneComponent.K2_GetComponentToWorld` (`self.DirtDropPoint`)) "Undefined" "MultiplyWithRoot" null null))
          (set `self.DirtDrop` _returnvalue_2))))
    (:`CastFailed`
      (bind _asbp_dirt_drop (cast `/Game/CleanHistory/BPs/BP_DirtDrop` OtherActor)
        (:`then`
          (`SceneComponent.SetRelativeScale3D` (`self.Scene`) (1.0 1.0 1.0))
          (`self.K2_DestroyActor` _asbp_dirt_drop))
        (:`CastFailed`
          (bind _ascorpse_members (cast `CorpseMembers` OtherActor))
          (`PrimitiveComponent.SetCollisionResponseToChannel` (`self.fill`) (`CorpseMembers.TraceChannelProperty` _ascorpse_members) "ECR_Ignore"))))))

(event `self.Box.OnComponentEndOverlap`
  (params (OverlappedComponent :type "PrimitiveComponent Object Reference") (OtherActor :type "Actor Object Reference") (OtherComp :type "PrimitiveComponent Object Reference") (OtherBodyIndex :type Integer)))

(fn `UserConstructionScript`)