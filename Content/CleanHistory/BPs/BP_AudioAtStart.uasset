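; BP_AudioAtStart is an actor that plays a sequence of four tutorial voice or sound clips as the level begins.
; On BeginPlay it waits a fixed initial delay, then plays each TutoSpawn sound in 2D in order.
; Between clips it waits for the current sound's duration plus a random pause, so the clips never overlap.
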(event `self.ReceiveBeginPlay`
  (bind _tutospawn1 (`self.TutoSpawn1`))
  (bind _tutospawn2 (`self.TutoSpawn2`))
  (bind _tutospawn3 (`self.TutoSpawn3`))
  (bind _tutospawn4 (`self.TutoSpawn4`))
  (`KismetSystemLibrary.Delay` 10.0)
  (`GameplayStatics.SpawnSound2D` _tutospawn1 1.0 1.0 0.0 null)
  (`KismetSystemLibrary.Delay` (+ (`SoundBase.Duration` _tutospawn1) (`KismetMathLibrary.RandomFloatInRange` 5.0 10.0)))
  (`GameplayStatics.SpawnSound2D` _tutospawn2 1.0 1.0 0.0 null)
  (`KismetSystemLibrary.Delay` (+ (`SoundBase.Duration` _tutospawn2) (`KismetMathLibrary.RandomFloatInRange` 5.0 10.0)))
  (`GameplayStatics.SpawnSound2D` _tutospawn3 1.0 1.0 0.0 null)
  (`KismetSystemLibrary.Delay` (+ (`SoundBase.Duration` _tutospawn3) (`KismetMathLibrary.RandomFloatInRange` 5.0 10.0)))
  (`GameplayStatics.SpawnSound2D` _tutospawn4 1.0 1.0 0.0 null)
  (`KismetSystemLibrary.Delay` (+ (`SoundBase.Duration` _tutospawn4) (`KismetMathLibrary.RandomFloatInRange` 5.0 10.0))))

(fn `UserConstructionScript`)