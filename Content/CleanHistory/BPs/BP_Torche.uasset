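; Torch that lights from a Brasero and spreads fire effects to props and burnables it touches.
; Box overlaps set IsBurning or attach fire ribbon Niagara systems, removed on a BP_Prop's death delegate.
; Tick hides FireMesh when its burnable counter runs out; while IsBurning, a reversed timeline shows it, then zeroes its scale and clears the flag.
; The counter is never decremented here, and older scale-animated ignite/extinguish logic is left disconnected.
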(event `CustomEvent`
  (params (DeltaSeconds :type "Float (single-precision)"))
  ;[1 1 1] More FeedBack on turn on and off
)

(event `self.ReceiveBeginPlay`
  (`SceneComponent.SetVisibility` (`self.FireMesh`) false true)
  (set `self.NbBurnbaleObject` 10000))

(event `self.CollisionBoxComponent.OnComponentBeginOverlap`
  (params (OverlappedComponent :type "PrimitiveComponent Object Reference") (OtherActor :type "Actor Object Reference") (OtherComp :type "PrimitiveComponent Object Reference") (OtherBodyIndex :type Integer) (bFromSweep :type Boolean) (SweepResult :type "HitResult Structure (by ref)"))
  (`|ExecutionSequence`
    (:`then_0`
      (cast `Brasero` OtherActor)
      (set `self.IsBurning` true))
    (:`then_1`
      ;[1 1 1] Spawn Particles IsBurning
      (bind _asbp_prop (cast `/Game/CleanHistory/BPs/BP_Prop` OtherActor)
        (:`then`
          (bind _returnvalue (`NiagaraFunctionLibrary.SpawnSystemAttached` "/Game/GA/fx/fire/ribon_fire/fire_ribbon.fire_ribbon" (`/Game/CleanHistory/BPs/BP_Prop.GrabComponent` _asbp_prop) "None" (0.0 0.0 0.0) (struct) "KeepRelativeOffset"))
          (add `Prop.OnDieDelegate` _asbp_prop (delegate `OnDieDelegate_Event`)))
        (:`CastFailed`
          (cast `IBurnable` OtherActor)
          (`NiagaraFunctionLibrary.SpawnSystemAttached` "/Game/GA/fx/fire/ribon_fire/fire_ribbon.fire_ribbon" (`Actor.RootComponent` OtherActor) "None" (0.0 0.0 0.0) (struct) "KeepRelativeOffset" true true "AutoRelease"))))))

(event `OnDieDelegate_Event`
  ;[1 1 1] Spawn Particles IsBurning
  (`ActorComponent.K2_DestroyComponent` (stale `self.CollisionBoxComponent.OnComponentBeginOverlap` _returnvalue)))

(event `self.ReceiveTick`
  (params (DeltaSeconds :type "Float (single-precision)"))
  (`|ExecutionSequence`
    (:`then_0`
      ;[1 1 1] Extinguishing
      (if (<= (`self.NbBurnbaleObject`) 0)
        (`SceneComponent.SetVisibility` (`self.FireMesh`) false true)))
    (:`then_1`
      ;[1 1 1] Ignite again
      (if (`self.IsBurning`)
        (if (`KismetSystemLibrary.IsValid` (`self.FireExstinctSound`))
          (`GameplayStatics.PlaySoundAtLocation` (`self.FireExstinctSound`) (0.0 0.0 0.0) (struct) 1.0 1.0 0.0 null null null null)
          (`Timeline|Timeline_1` :!via `ReverseFromEnd` :!label _label
            (:`Update`
              (`SceneComponent.SetVisibility` (`self.FireMesh`) true true))
            (:`Finished`
              (`SceneComponent.SetWorldScale3D` (`self.FireMesh`) (0.0 0.0 0.0))
              (set `self.IsBurning` false)))
          (else
            (goto _label :!via `ReverseFromEnd`)))))))

(fn `Get Grab Component Transform`
  (returns (GrabComponent :type "Transform Structure"))
  (return))

(fn `UserConstructionScript`)