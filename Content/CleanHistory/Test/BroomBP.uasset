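; Broom actor Blueprint, in a test folder, that delegates drawing and washing to a DrawAndWash component.
; On BeginPlay it adds three root points to that component's RootTarget list, allowing multiple raycasts.
; CleanBroom cleans the broom by a configurable wash percentage, while BPCleanBroom passes a fixed amount.
; A helper exposes the GrabComponent's world transform.
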(event `self.ReceiveBeginPlay`
  (bind _roottarget (`/Game/CleanHistory/Test/DrawAndWash.RootTarget` (`self.DrawAndWash`)))
  ;[1 1 1] Add all the root to the root target (allow multiple raycast)
  (`|ExecutionSequence`
    (:`then_0`
      (`KismetArrayLibrary.Array_Add` _roottarget (`self.Root 1`)))
    (:`then_1`
      (`KismetArrayLibrary.Array_Add` _roottarget (`self.Root 2`)))
    (:`then_2`
      (`KismetArrayLibrary.Array_Add` _roottarget (`self.Root 3`)))))

(event `self.CleanBroom`
  (`/Game/CleanHistory/Test/DrawAndWash.CleanBroom` (`self.DrawAndWash`) (`self.PercentageCleanedByWash`)))

(fn `BPCleanBroom`
  (`/Game/CleanHistory/Test/DrawAndWash.CleanBroom` (`self.DrawAndWash`) 25.0))

(fn `Get Grab Component Transform`
  (returns (GrabComponent :type "Transform Structure"))
  (return (`SceneComponent.K2_GetComponentToWorld` (`self.GrabComponent`))))

(fn `UserConstructionScript`)