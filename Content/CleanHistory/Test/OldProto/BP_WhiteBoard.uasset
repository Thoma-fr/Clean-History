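; Prototype whiteboard actor that can be drawn on and erased at runtime.
; On BeginPlay it creates board and marker material instances plus a canvas render target, which feeds the board material on the Cube.
; Draw and Wash stamp the marker material into that target at a given 2D position, in white or black respectively.
; Wash also enlarges or sets the brush size, which Draw never resets.
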(event `self.ReceiveBeginPlay`
  ;[1 0.1948 0.4074] BeginPlay
  (`|ExecutionSequence`
    (:`then_0`
      ;;[1 1 1] current material instance
      (bind _returnvalue (`KismetMaterialLibrary.CreateDynamicMaterialInstance` "/Game/CleanHistory/Test/OldProto/Materials/M_WhiteBoard.M_WhiteBoard"))
      (bind _output_get (set `self.Whiteboard` _returnvalue))
      (`PrimitiveComponent.SetMaterial` (`self.Cube`) 0 _output_get))
    (:`then_1`
      ;;[1 1 1] Marker Instance
      (bind _returnvalue_2 (`KismetMaterialLibrary.CreateDynamicMaterialInstance` "/Game/CleanHistory/Test/OldProto/Materials/M_Mark.M_Mark"))
      (set `self.WhiteBoardMarker_MI` _returnvalue_2))
    (:`then_2`
      ;;[1 1 1] Create a Render Target Instance
      (bind _output_get_2 (set `self.RenderTarget` "/Game/CleanHistory/Test/OldProto/RT_WhiteBoard.RT_WhiteBoard"))
      (bind _returnvalue_3 (`CanvasRenderTarget2D.CreateCanvasRenderTarget2D` _output_get_2 "/Script/Engine.CanvasRenderTarget2D" 512 512))
      (set `self.CurrentRenderTarget` _returnvalue_3))
    (:`then_3`
      ;;[1 1 1] Set the current render target to the current material to allow the lerp
      (`MaterialInstanceDynamic.SetTextureParameterValue` (`self.Whiteboard`) "CurrentRenderTarget" (`self.CurrentRenderTarget`)))))

(event `Draw`
  (params (`location to draw` :type "Vector2D Structure"))
  (bind _whiteboardmarker_mi (`self.WhiteBoardMarker_MI`))
  ;[1 1 1] Draw
  (`MaterialInstanceDynamic.SetVectorParameterValue` _whiteboardmarker_mi "DrawLocation" (`KismetMathLibrary.Conv_VectorToLinearColor` (`KismetMathLibrary.Conv_Vector2DToVector` `location to draw`)))
  (`MaterialInstanceDynamic.SetVectorParameterValue` _whiteboardmarker_mi "CurrentColor" (struct :`R` 1.0 :`G` 1.0 :`B` 1.0 :`A` 1.0))
  (`KismetRenderingLibrary.DrawMaterialToRenderTarget` (`self.CurrentRenderTarget`) _whiteboardmarker_mi))

(event `Wash`
  (params (PosToWash :type "Vector2D Structure"))
  (bind _whiteboardmarker_mi (`self.WhiteBoardMarker_MI`))
  ;[1 1 1] Wash
  (`|ExecutionSequence`
    (:`then_0`
      (`MaterialInstanceDynamic.SetVectorParameterValue` _whiteboardmarker_mi "DrawLocation" (`KismetMathLibrary.Conv_VectorToLinearColor` (`KismetMathLibrary.Conv_Vector2DToVector` PosToWash)))
      (`MaterialInstanceDynamic.SetVectorParameterValue` _whiteboardmarker_mi "CurrentColor" (struct :`A` 1.0))
      (`MaterialInstanceDynamic.SetScalarParameterValue` _whiteboardmarker_mi "DrawSize" 0.15))
    (:`then_1`
      (`KismetRenderingLibrary.DrawMaterialToRenderTarget` (`self.CurrentRenderTarget`) _whiteboardmarker_mi))))

(fn `UserConstructionScript`)