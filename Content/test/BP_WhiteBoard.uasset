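; BP_WhiteBoard is a whiteboard that can be drawn on and wiped at given 2D positions.
; BeginPlay creates dynamic marker and washer materials and clears the RT_WhiteBoard and Mask render targets to black.
; Draw and Wash pass the position through the DrawLocation parameter and render their material into RT_WhiteBoard.
; Draw also stamps into Mask, which Wash leaves untouched.
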(event `self.ReceiveBeginPlay`
  (bind _returnvalue (`KismetMaterialLibrary.CreateDynamicMaterialInstance` "/Game/test/M_Mark.M_Mark"))
  (set `self.WhiteBoardMarker_MI` _returnvalue)
  (bind _returnvalue_2 (`KismetMaterialLibrary.CreateDynamicMaterialInstance` "/Game/test/M_Clean.M_Clean"))
  (set `self.WhiteBoardWasher_MI` _returnvalue_2)
  (`KismetRenderingLibrary.ClearRenderTarget2D` "/Game/test/RT_WhiteBoard.RT_WhiteBoard")
  (`KismetRenderingLibrary.ClearRenderTarget2D` "/Game/test/Mask.Mask"))

(event `Draw`
  (params (`location to draw` :type "Vector2D Structure"))
  (bind _whiteboardmarker_mi (`self.WhiteBoardMarker_MI`))
  (`MaterialInstanceDynamic.SetVectorParameterValue` _whiteboardmarker_mi "DrawLocation" (`KismetMathLibrary.Conv_VectorToLinearColor` (`KismetMathLibrary.Conv_Vector2DToVector` `location to draw`)))
  (`KismetRenderingLibrary.DrawMaterialToRenderTarget` "/Game/test/RT_WhiteBoard.RT_WhiteBoard" _whiteboardmarker_mi)
  (`KismetRenderingLibrary.DrawMaterialToRenderTarget` "/Game/test/Mask.Mask" _whiteboardmarker_mi))

(event `Wash`
  (params (PosToWash :type "Vector2D Structure"))
  (bind _whiteboardwasher_mi (`self.WhiteBoardWasher_MI`))
  (`MaterialInstanceDynamic.SetVectorParameterValue` _whiteboardwasher_mi "DrawLocation" (`KismetMathLibrary.Conv_VectorToLinearColor` (`KismetMathLibrary.Conv_Vector2DToVector` PosToWash)))
  (`KismetRenderingLibrary.DrawMaterialToRenderTarget` "/Game/test/RT_WhiteBoard.RT_WhiteBoard" _whiteboardwasher_mi))

(fn `UserConstructionScript`)