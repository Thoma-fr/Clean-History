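; Angel_BP is an angel actor whose static mesh rises while turning to face the player.
; On BeginPlay, the Size timeline drives the mesh's uniform world scale from its track value.
; Each tick, the mesh moves up in world Z by Speed without delta-time scaling and yaws toward the player pawn, with pitch and roll held at zero.
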(event `self.ReceiveBeginPlay`
  (bind (_direction _newtrack_0) (`Timeline|size`)
    (:`Update`
      (`SceneComponent.SetWorldScale3D` (`self.StaticMesh`) (* (`KismetMathLibrary.Vector_One`) _newtrack_0 0.25)))))

(event `self.ReceiveTick`
  (params (DeltaSeconds :type "Float (single-precision)"))
  (bind _staticmesh (`self.StaticMesh`))
  (bind _staticmesh_2 (`self.StaticMesh`))
  (bind (_returnvalue_roll _returnvalue_pitch _returnvalue_yaw) (`KismetMathLibrary.BreakRotator` (`KismetMathLibrary.FindLookAtRotation` (`SceneComponent.K2_GetComponentLocation` _staticmesh) (`self.K2_GetActorLocation` (`GameplayStatics.GetPlayerPawn` 0)))))
  (`SceneComponent.K2_SetWorldLocation` _staticmesh_2 (+ (`SceneComponent.K2_GetComponentLocation` _staticmesh_2) (`KismetMathLibrary.MakeVector` 0.0 0.0 (`self.Speed`))) false false)
  (`SceneComponent.K2_SetWorldRotation` _staticmesh (`KismetMathLibrary.MakeRotator` 0.0 0.0 _returnvalue_yaw) false false))

(fn `UserConstructionScript`)